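; BP_AI_Spawner_Ranged is a spawner that keeps ranged enemies in play at the location of its Billboard component.
; Every Tick it counts all BP_enemy_Ranged actors, allowing a spawn while the count is at or below MaxInPlay.
; The spawn event waits on a fixed Delay, which paces the per-frame calls, then plays an explosion effect and spawns the enemy with BT_Enemy_Ranged.
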(event `self.ReceiveBeginPlay`)

(event `self.ReceiveTick`
  (params (DeltaSeconds :type "Float (single-precision)"))
  (bind _outactors (`GameplayStatics.GetAllActorsOfClass` "/Game/Characters/AI/enemies/BP_enemy_Ranged.BP_enemy_Ranged_C"))
  (set `self.CanSpawn` (<= (`KismetArrayLibrary.Array_Length` _outactors) (`self.Max in Play`)))
  (`self.Spawn enemy`))

(event `Spawn enemy`
  (bind _billboard (`self.Billboard`))
  (bind _returnvalue (`SceneComponent.K2_GetComponentLocation` _billboard))
  (if (`self.CanSpawn`)
    (`KismetSystemLibrary.Delay` 5.0)
    (`GameplayStatics.SpawnEmitterAtLocation` "/Game/StarterContent/Particles/P_Explosion.P_Explosion" _returnvalue)
    (`AIBlueprintHelperLibrary.SpawnAIFromClass` "/Game/Characters/AI/enemies/BP_enemy_Ranged.BP_enemy_Ranged_C" "/Game/Characters/AI/enemies/AI_Logic/BehaviorTrees/BT_Enemy_Ranged.BT_Enemy_Ranged" _returnvalue (`SceneComponent.K2_GetComponentRotation` _billboard) false null)))

(fn `UserConstructionScript`)