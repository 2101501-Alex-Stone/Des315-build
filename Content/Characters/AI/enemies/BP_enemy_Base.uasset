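; Base enemy AI character with a health bar, healing, arc-launched jumps, a player-notice montage, and range and speed helpers.
; Tick refreshes the bar from StatusComponent and calls DeathControl every frame health is at zero or below, with no one-shot guard.
; DeathControl awards random score, ragdolls the mesh, then unequips and destroys the actor after a delay.
; TraceAttack sphere-traces for the player, using HitActors to prevent repeat damage.
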(event `self.ReceiveBeginPlay`
  (bind _output_get (set `self.UI HPBar Enemy Ref` (cast `/Game/UI/Enemies/UI_HPBarEnemy` (`WidgetComponent.GetUserWidgetObject` (`self.EnemyHealthBar`)) :!pure true)))
  (`/Game/UI/Enemies/UI_HPBarEnemy.RefershHealthBar` _output_get (`self.Status_Component`)))

(event `self.ReceiveTick`
  (params (DeltaSeconds :type "Float (single-precision)"))
  (bind _status_component (`self.Status_Component`))
  (`/Game/UI/Enemies/UI_HPBarEnemy.RefershHealthBar` (`self.UI HPBar Enemy Ref`) _status_component)
  (if (<= (`/Game/DamageSystem/BP_Status_Component.CurrentHealth` _status_component) 0.0)
    (`self.DeathControl`)))

(event `self.JumpToDestination`
  (params (Destination :type "Vector Structure"))
  ;[0.009047 0.1723 1] Jump func
  (bind _outlaunchvelocity (`GameplayStatics.SuggestProjectileVelocity_CustomArc` (`self.K2_GetActorLocation`) (`KismetMathLibrary.MakeVector` (.x Destination) (.y Destination) (+ (.z Destination) (`self.JumpHeight`)))))
  (`self.LaunchCharacter` _outlaunchvelocity true true))

(event `self.NoticePlayer`
  ;[0.004949 0.2185 1] Notice Player
  (`|PlayMontage` (`self.Mesh`) "/Game/Characters/AI/Assets/AM_Notice_Player.AM_Notice_Player"))

(event `DeathControl`
  (bind _mesh (`self.Mesh`))
  ;[0.03439 0.311 1] Death control
  (`Widget.SetVisibility` (`self.UI HPBar Enemy Ref`) "Hidden")
  (bind _asbp_third_person_game_mode (cast `/Game/ThirdPerson/Blueprints/BP_ThirdPersonGameMode` (`GameplayStatics.GetGameMode`)))
  (`/Game/UI/GameMode/UI_Calc_Component.AddPlayerScore` (`/Game/ThirdPerson/Blueprints/BP_ThirdPersonGameMode.UI_Calc_Component` _asbp_third_person_game_mode) (`KismetMathLibrary.Conv_IntToDouble` (`KismetMathLibrary.RandomIntegerInRange` 10 15)))
  (`PrimitiveComponent.SetSimulatePhysics` _mesh true)
  (`PrimitiveComponent.SetCollisionEnabled` _mesh "QueryAndPhysics")
  (`KismetSystemLibrary.Delay` 5.0)
  (`self.UnequipWeapon`)
  (`self.K2_DestroyActor`))

(event `/Game/Characters/AI/enemies/AI_Logic/BPI_AI.Heal`
  (params (Percent :type "Float (double-precision)"))
  (bind _status_component (`self.Status_Component`))
  (`/Game/DamageSystem/BP_Status_Component.IncreaseHealth` _status_component (* Percent (`/Game/DamageSystem/BP_Status_Component.MaxHealth` _status_component))))

(event `/Game/Characters/AI/enemies/AI_Logic/BPI_AI.JumpTo`
  (params (destination :type "Vector Structure"))
  (bind _outlaunchvelocity (`GameplayStatics.SuggestProjectileVelocity_CustomArc` (`self.K2_GetActorLocation`) (`KismetMathLibrary.MakeVector` (.x destination) (.y destination) (+ (.z destination) (`self.JumpHeight`)))))
  (`self.LaunchCharacter` _outlaunchvelocity))

(fn `Check in Range`
  (returns (inRange :type Boolean))
  (return (< (`self.GetDistanceTo` (`GameplayStatics.GetPlayerCharacter` 0)) (`self.AttackRange`))))

(fn `Get maxHealth`
  (returns (MaxHealth :type "Float (double-precision)"))
  (return (`/Game/DamageSystem/BP_Status_Component.MaxHealth` (`self.Status_Component`))))

(fn `GetCurrentHealth`
  (returns (currentHealth :type "Float (double-precision)"))
  (return (`/Game/DamageSystem/BP_Status_Component.CurrentHealth` (`self.Status_Component`))))

(fn `GetIdealRange`
  (returns (AttackRadius :type "Float (double-precision)") (DefendRadius :type "Float (double-precision)"))
  (return 50.0 350.0))

(fn `SetMovmentSpeed`
  (params (Speed :type "/Game/Characters/AI/enemies/AI_Logic/Enums/E_MovmentSpeed Enum" :default "NewEnumerator0"))
  (returns (SpeedValue :type "Float (double-precision)"))
  (bind _output_get (set `CharacterMovementComponent.MaxWalkSpeed` (select `/Game/Characters/AI/enemies/AI_Logic/Enums/E_MovmentSpeed` Speed :`NewEnumerator1` (`KismetMathLibrary.RandomFloatInRange` 100.0 150.0) :`NewEnumerator2` (`KismetMathLibrary.RandomFloatInRange` 300.0 350.0) :`NewEnumerator3` (`KismetMathLibrary.RandomFloatInRange` 500.0 550.0) :!type "Float (single-precision)") (`self.CharacterMovement`)))
  (return _output_get))

(fn `TraceAttack`
  (params (Start :type "Vector Structure") (end :type "Vector Structure"))
  (bind _outhits (`KismetSystemLibrary.SphereTraceMulti` Start end 10.0 "TraceTypeQuery3"))
  (if true
    (for _array_element _outhits
      (bind (_bblockinghit _binitialoverlap _time _distance _location _impactpoint _normal _impactnormal _physmat _hitactor) (`GameplayStatics.BreakHitResult` _array_element))
      (if (and (`KismetMathLibrary.ClassIsChildOf` (`GameplayStatics.GetObjectClass` _hitactor) "/Game/RuWork/Player/BP_PlayerCharacter.BP_PlayerCharacter_C") (not (`KismetArrayLibrary.Array_Contains` (`self.HitActors`) _hitactor)))
        (`KismetArrayLibrary.Array_Add` (`self.HitActors`) _hitactor)
        (bind _wasdamaged (message `/Game/DamageSystem/BPI_Damagable.TakeDamage` _hitactor (make `/Game/DamageSystem/S_DamageInfo` 20.0 "NewEnumerator1" "NewEnumerator1")))
        (if _wasdamaged
          (`GameplayStatics.SpawnEmitterAtLocation` "/Game/StarterContent/Particles/P_Explosion.P_Explosion" _location))
        (return)))))

(fn `UserConstructionScript`)