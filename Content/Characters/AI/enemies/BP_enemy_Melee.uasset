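; Melee enemy character that dual-wields swords, with equip, unequip, attack and hit-detection events plus attack and defend ranges.
; Equipping plays a notice-player montage whose notify spawns both swords on the arm sockets; unequipping destroys them.
; Attacks alternate between two stab montages and signal their end on completion or interruption.
; Hit detection runs a looping timer that traces along both arms, clearing hit actors when each trace window starts.
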(event `/Game/Characters/AI/enemies/AI_Logic/BPI_AI.EquipWeapon`
  (bind _returnvalue (`self.GetTransform`))
  ;[0 0.09116 1] Equip Weapon
  (bind _notifyname (`|PlayMontage` (`self.Mesh`) "/Game/Characters/AI/Assets/AM_Notice_Player.AM_Notice_Player")
    (:`OnNotifyBegin`
      (switch `name` _notifyname
        (:`WeaponSpawn`
          (bind _returnvalue_2 (`|SpawnActorFromClass` "/Game/Characters/AI/Weapons/BP_Sword0.BP_Sword0_C" _returnvalue "Undefined" "MultiplyWithRoot" null null))
          (`KismetArrayLibrary.Array_Add` (`self.EquippedWeapons`) _returnvalue_2)
          (`self.K2_AttachToComponent` _returnvalue_2 (`self.Mesh`) "LeftArmSocket" "SnapToTarget" "SnapToTarget" "SnapToTarget" true)
          (bind _returnvalue_3 (`|SpawnActorFromClass` "/Game/Characters/AI/Weapons/BP_Sword1.BP_Sword1_C" _returnvalue "Undefined" "MultiplyWithRoot" null null))
          (`KismetArrayLibrary.Array_Add` (`self.EquippedWeapons`) _returnvalue_3)
          (`self.K2_AttachToComponent` _returnvalue_3 (`self.Mesh`) "RightArmSocket" "SnapToTarget" "SnapToTarget" "SnapToTarget" true)
          (set `self.IsWieldingWeapon` true))))))

(event `/Game/Characters/AI/enemies/AI_Logic/BPI_AI.UnequipWeapon`
  ;[0.009047 0.1723 1] Unequip Weapon
  (for _array_element (`self.EquippedWeapons`)
    (`self.K2_DestroyActor` _array_element))
  (set `self.IsWieldingWeapon` false)
  (`self.OnUnequipWeapon`))

(event `/Game/Characters/AI/enemies/AI_Logic/BPI_AI.DefaultAttack`
  ;[0 0.0615 1] Default Attack
  (if (> (`self.AttackCount`) 1)
    (set `self.AttackCount` 0))
  (if (== (`self.AttackCount`) 0)
    (`|PlayMontage` (`self.Mesh`) "/Game/Characters/AI/Assets/Animations/Attacks/Montage_Stab_1.Montage_Stab_1"
      (:`OnCompleted`
        _)
      (:`OnInterrupted`
        _))
    (else
      (`|PlayMontage` (`self.Mesh`) "/Game/Characters/AI/Assets/Animations/Attacks/Montage_Stab2.Montage_Stab2"
        (:`OnCompleted`
          _)
        (:`OnInterrupted`
          _))))
  (set `self.AttackCount` (+ (`self.AttackCount`) 1))
  (`self.OnAttackEnd`))

(event `StopLineTrace`
  ;[0.01173 0.0532 1] Hit Detection
  (`KismetSystemLibrary.K2_ClearAndInvalidateTimerHandle` (stale `TriggerLineTrace` _returnvalue)))

(event `TriggerLineTrace`
  ;[0.01173 0.0532 1] Hit Detection
  (`KismetArrayLibrary.Array_Clear` (`self.HitActors`))
  (bind _returnvalue (`KismetSystemLibrary.K2_SetTimerDelegate` (delegate `ApplyLineTrace`) 0.01 true)))

(event `ApplyLineTrace`
  (bind _mesh (`self.Mesh`))
  (bind _mesh_2 (`self.Mesh`))
  ;[0.01173 0.0532 1] Hit Detection
  (`self.TraceAttack` (`SceneComponent.GetSocketLocation` _mesh_2 "LeftArmSocket") (`SceneComponent.GetSocketLocation` _mesh_2 "LeftHandSocket"))
  (`self.TraceAttack` (`SceneComponent.GetSocketLocation` _mesh "RightArmSocket") (`SceneComponent.GetSocketLocation` _mesh "RightHandSocket")))

(fn `GetIdealRange`
  (returns (AttackRadius :type "Float (double-precision)") (DefendRadius :type "Float (double-precision)"))
  (return (`self.AttackRadius`) (`self.DefendRadius`)))

(fn `UserConstructionScript`
  (`parent.UserConstructionScript`))