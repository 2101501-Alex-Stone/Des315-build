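; Ranged enemy character that spawns a gun into its right hand on BeginPlay and attacks by firing energy projectiles.
; DefaultAttack plays a rifle montage whose notify spawns a projectile aimed at the AI controller's AttackTarget, then signals attack end on completion or interruption.
; Projectile impacts are bound back to the enemy, which damages only the player through its StatusComponent.
; It also supplies randomized walk speeds per movement state and attack/defend radii.
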(event `self.ReceiveBeginPlay`
  (`parent.ReceiveBeginPlay`)
  (`self.EquipWeapon`))

(event `/Game/Characters/AI/enemies/AI_Logic/BPI_AI.EquipWeapon`
  (bind _returnvalue (`|SpawnActorFromClass` "/Game/Characters/AI/Weapons/BP_Arm_Gun.BP_Arm_Gun_C" (`self.GetTransform`) "Undefined" "MultiplyWithRoot" null null))
  (`KismetArrayLibrary.Array_Add` (`self.EquippedWeapons`) _returnvalue)
  (`self.K2_AttachToComponent` _returnvalue (`self.Mesh`) "RightHandSocket" "SnapToTarget" "SnapToTarget" "SnapToTarget" true)
  (set `self.IsWieldingWeapon` true))

(event `/Game/Characters/AI/enemies/AI_Logic/BPI_AI.DefaultAttack`
  (bind _notifyname (`|PlayMontage` (`self.Mesh`) "/Game/Characters/AI/Assets/Animations/Attacks/Montage_Fire_Rifle.Montage_Fire_Rifle")
    (:`OnCompleted`
      (`self.OnAttackEnd` :!label _label))
    (:`OnInterrupted`
      (goto _label))
    (:`OnNotifyBegin`
      (switch `name` _notifyname
        (:`Fire`
          (bind _asaic_enemy_base (cast `/Game/Characters/AI/enemies/AI_Logic/AIC_Enemy_Base` (`AIBlueprintHelperLibrary.GetAIController` self)))
          (bind _returnvalue (`|SpawnActorFromClass` "/Game/Characters/AI/Weapons/Projectiles/BP_Projectile_Energy.BP_Projectile_Energy_C" (`SceneComponent.K2_GetComponentToWorld` (`self.Scene`)) "Undefined" "MultiplyWithRoot" self 500.0 0.0 (`/Game/Characters/AI/enemies/AI_Logic/AIC_Enemy_Base.Attack Target` _asaic_enemy_base) false null))
          (add `/Game/Characters/AI/Weapons/Projectiles/BP_Projectile_Base.OnProjectileImpact` _returnvalue (delegate `DamageTarget`))
          (`PrimitiveComponent.IgnoreActorWhenMoving` (`self.CapsuleComponent`) null true))))))

(event `DamageTarget`
  (params (OtherActor :type "Actor Object Reference") (Hit :type "HitResult Structure"))
  (bind _returnvalue (`GameplayStatics.GetActorOfClass` "/Game/RuWork/Player/BP_PlayerCharacter.BP_PlayerCharacter_C"))
  (if (== _returnvalue (`.HitActor` (`GameplayStatics.BreakHitResult` Hit)))
    (`/Game/DamageSystem/BP_Status_Component.DecreaseHealth` (`/Game/RuWork/Player/BP_PlayerCharacter.Status_Component` _returnvalue) (`self.AttackDamage`))))

(fn `GetIdealRange`
  (returns (AttackRadius :type "Float (double-precision)") (DefendRadius :type "Float (double-precision)"))
  (return (`self.AttackRadius`) (`self.DefendRadius`)))

(fn `SetMovmentSpeed`
  (params (Speed :type "/Game/Characters/AI/enemies/AI_Logic/Enums/E_MovmentSpeed Enum" :default "NewEnumerator0"))
  (returns (SpeedValue :type "Float (double-precision)"))
  (bind _output_get (set `CharacterMovementComponent.MaxWalkSpeed` (select `/Game/Characters/AI/enemies/AI_Logic/Enums/E_MovmentSpeed` Speed :`NewEnumerator1` (`KismetMathLibrary.RandomFloatInRange` 200.0 250.0) :`NewEnumerator2` (`KismetMathLibrary.RandomFloatInRange` 350.0 400.0) :`NewEnumerator3` (`KismetMathLibrary.RandomFloatInRange` 500.0 550.0) :!type "Float (single-precision)") (`self.CharacterMovement`)))
  (return _output_get))

(fn `UserConstructionScript`
  (`parent.UserConstructionScript`))