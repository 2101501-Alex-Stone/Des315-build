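; BP_Status_Component is an actor component that tracks health, death and damage handling for its owner.
; TakeDamage passes incoming damage info through the CanBeDamaged macro, which checks death, invincibility and blocking to block, apply or ignore the hit.
; Blocked, death and damage response events are broadcast, the last only when the owner is interruptible or interruption is forced.
; Separate functions adjust health directly, with only increases clamped.
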(fn `DecreaseHealth`
  (params (Amount :type "Float (double-precision)"))
  (returns (`Is Dead` :type Boolean))
  (bind _output_get (set `self.CurrentHealth` (- (`self.CurrentHealth`) Amount)))
  (return (<= _output_get 0.0)))

(fn `IncreaseHealth`
  (params (Amount :type "Float (double-precision)"))
  (returns (NewAmount :type "Float (double-precision)"))
  (if (not (`self.IsDead`))
    (bind _output_get (set `self.CurrentHealth` (`KismetMathLibrary.FClamp` (+ Amount (`self.CurrentHealth`)) 0.0 (`self.MaxHealth`))))
    (return _output_get)))

(fn `TakeDamage`
  (params (DamageInfo :type "/Game/DamageSystem/S_DamageInfo Structure"))
  (returns (WasDamaged :type Boolean))
  (bind (_amount _damagetype _damagereaction _shoulddamageinvincible _canbeblocked _canbeparried _canbedodged _shouldforceinterupt) (break `/Game/DamageSystem/S_DamageInfo` DamageInfo))
  (`self.CanBeDamaged` _shoulddamageinvincible _canbeblocked
    (:`BlockDamage`
      (`self.OnBlocked`)
      (return false))
    (:`DoDamage`
      (bind _output_get (set `self.CurrentHealth` (- (`self.CurrentHealth`) _amount)))
      (if (<= _output_get 0.0)
        (set `self.IsDead` true)
        (`self.OnDeath`)
        (return true)
        (elif (or (`self.IsInteruptable`) _shouldforceinterupt)
          (`self.OnDamageResponse` _damagereaction)
          (return true))))
    (:`NoDamage`
      (return false))))