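; Explosive barrel hazard that blows up when its mesh is hit by a Character while the barrel actor is moving.
; On hit, it requires any signed axis of its own velocity to exceed a small threshold, so negative-direction motion alone does not qualify.
; It then spawns a scaled-up explosion particle at the mesh, fires a RadialForce impulse and destroys itself.
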(event `self.SM_ExplodeBarrel.OnComponentHit`
  (params (HitComponent :type "PrimitiveComponent Object Reference") (OtherActor :type "Actor Object Reference") (OtherComp :type "PrimitiveComponent Object Reference") (NormalImpulse :type "Vector Structure") (Hit :type "HitResult Structure (by ref)"))
  (bind (_returnvalue_x _returnvalue_y _returnvalue_z) (`KismetMathLibrary.BreakVector` (`self.GetVelocity`)))
  (cast `Character` OtherActor)
  (if (or (> _returnvalue_x 5.0) (> _returnvalue_y 5.0) (> _returnvalue_z 5.0))
    (`GameplayStatics.SpawnEmitterAtLocation` "/Game/StarterContent/Particles/P_Explosion.P_Explosion" (`SceneComponent.K2_GetComponentLocation` (`self.SM_ExplodeBarrel`)) (struct) (4.0 4.0 4.0))
    (`RadialForceComponent.FireImpulse` (`self.RadialForce`))
    (`self.K2_DestroyActor`)))

(fn `UserConstructionScript`)