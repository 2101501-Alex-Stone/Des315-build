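; Player 1 character that spawns a socket-attached axe guitar, adds its HUD and fights with melee and push abilities.
; Attacks step through montages by combo count, while HitDetection sphere-traces along the axe and destroys any BP_PlayerCharacter hit.
; Force ability scales an aimed sphere-trace push with hold time, briefly enabling capsule physics on hit characters.
; Special charges a radius, then pushes surrounding components away using impact normals.
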(event `self.ReceiveBeginPlay`
  (`parent.ReceiveBeginPlay`)
  (bind _returnvalue (`|SpawnActorFromClass` "/Game/RuWork/Melee/Axe/BP_AxeGuitar.BP_AxeGuitar_C" (`self.GetTransform`) "Undefined" "MultiplyWithRoot" null null))
  (bind _output_get (set `self.AxeGuitar` _returnvalue))
  (`self.K2_AttachToComponent` _output_get (`self.Mesh`) "AxeHand" "SnapToTarget" "SnapToTarget" "SnapToTarget" true)
  ;[0 0.07882 1] Adds UI to first player
  (cast `PlayerController` (`self.GetController`))
  (bind _returnvalue_2 (`|CreateWidget` "/Game/UI/Players/Player1HUD_Widgit.Player1HUD_Widgit_C"))
  (bind _output_get_2 (set `self.HUDRef` _returnvalue_2))
  (`UserWidget.AddToPlayerScreen` _output_get_2 0))

(event `self.ReceiveTick`
  (params (DeltaSeconds :type "Float (single-precision)")))

(event `EnhancedInput|/Game/Combat/Inputs/IA_PlayerAttack`
  (params (ActionValue :type Boolean) (ElapsedSeconds :type "Float (double-precision)") (TriggeredSeconds :type "Float (double-precision)") (InputAction :type "InputAction Object Reference" :default "/Game/Combat/Inputs/IA_PlayerAttack.IA_PlayerAttack"))
  ;[1 0.4072 0] Melee Attack - Combo attacks with hit detection and various animations
  (:`Started`
    (if (not (`self.IsAttacking`))
      (set `self.IsAttacking` true)
      (`|PlayMontage` (`self.Mesh`) (select `int` (`self.AttackCount`) :`0` "/Game/RuWork/Animations/NewAnim/NewAnimMontage.NewAnimMontage" :`1` null :`2` null :!type "AnimMontage Object Reference")
        (:`then`
          (`/Engine/EditorBlueprintResources/StandardMacros.IncrementInt` (`self.AttackCount`)))
        (:`OnCompleted`
          (set `self.IsAttacking` false :!label _label)
          (set `self.AttackCount` 0))
        (:`OnInterrupted`
          (`KismetSystemLibrary.RetriggerableDelay` 1.8)
          (goto _label))))))

(event `EnhancedInput|/Game/Combat/Inputs/IA_ForceAbility`
  (params (ActionValue :type Boolean) (ElapsedSeconds :type "Float (double-precision)") (TriggeredSeconds :type "Float (double-precision)") (InputAction :type "InputAction Object Reference" :default "/Game/Combat/Inputs/IA_ForceAbility.IA_ForceAbility"))
  (bind _returnvalue (* ElapsedSeconds 400.0))
  (bind _returnvalue_2 (`SceneComponent.K2_GetComponentLocation` (`self.RootComponent`)))
  (bind _returnvalue_3 (* (`self.RegisterDistance`) (`self.Multiplier`)))
  (bind _returnvalue_4 (* (`KismetMathLibrary.GetForwardVector` (`self.GetBaseAimRotation`)) (select `bool` (<= _returnvalue_3 1000.0) :`false` 1000.0 :`true` _returnvalue_3)))
  ;[0.9 0.1664 0] Pushing Ability -> Activates when pressed and forces enemies away
  (:`Triggered`
    (if (>= (- (`KismetSystemLibrary.GetGameTimeInSeconds`) (`self.Last Cast Time`)) 0.5)
      _))
  (:`Ongoing`
    (set `self.Multiplier` (select `bool` (>= ElapsedSeconds 1.0) :`false` 1.0 :`true` ElapsedSeconds :!type "Float (single-precision)"))
    (set `self.AbilityRadius` (select `bool` (<= _returnvalue 499.0) :`false` 500.0 :`true` _returnvalue :!type "Float (single-precision)"))
    (set `self.PushDirection` (* _returnvalue_4 (* (`self.Multiplier`) (`self.PushForce`))))
    (bind _output_get (set `self.StartVal` _returnvalue_2))
    (bind _output_get_2 (set `self.EndVal` (+ _returnvalue_2 _returnvalue_4)))
    (`KismetSystemLibrary.SphereTraceMulti` :`Start` _output_get :`End` _output_get_2 :`Radius` 250.0 :`TraceChannel` "TraceTypeQuery4" :`DrawDebugType` "ForOneFrame"))
  (:`Completed`
    (bind _outhits (`KismetSystemLibrary.SphereTraceMulti` :`Start` (`self.StartVal`) :`End` (`self.EndVal`) :`Radius` 250.0 :`TraceChannel` "TraceTypeQuery4" :`DrawDebugType` "ForDuration"))
    (for _array_element _outhits
      (bind (_bblockinghit _binitialoverlap _time _distance _location _impactpoint _normal _impactnormal _physmat _hitactor _hitcomponent) (`GameplayStatics.BreakHitResult` _array_element))
      (if (`KismetMathLibrary.ClassIsChildOf` (`GameplayStatics.GetObjectClass` _hitactor) "/Script/Engine.Character")
        (bind _returnvalue_5 (`self.GetComponentByClass` _hitactor "/Script/Engine.CapsuleComponent"))
        (`PrimitiveComponent.SetSimulatePhysics` _returnvalue_5 true)
        (`PrimitiveComponent.AddForce` _returnvalue_5 (`self.PushDirection`) "None" false)
        (`KismetSystemLibrary.Delay` 0.2)
        (`PrimitiveComponent.SetSimulatePhysics` _returnvalue_5 false)
        (set `self.Last Cast Time` (`KismetSystemLibrary.GetGameTimeInSeconds`))
        (else
          (`PrimitiveComponent.AddForce` _hitcomponent (`self.PushDirection`) "None" false))))))

(event `EnhancedInput|/Game/Combat/Inputs/IA_Special`
  (params (ActionValue :type Boolean) (ElapsedSeconds :type "Float (double-precision)") (TriggeredSeconds :type "Float (double-precision)") (InputAction :type "InputAction Object Reference" :default "/Game/Combat/Inputs/IA_Special.IA_Special"))
  (bind _returnvalue (* ElapsedSeconds 400.0))
  (bind _returnvalue_2 (`SceneComponent.K2_GetComponentLocation` (`self.CapsuleComponent`)))
  ;[0.9 0.1664 0] Push Repulse -> Charge up ability to released an AoE push affect that builds in both range and power the longer it is held
  (:`Started`
    (if (not (`self.IsUsingAbility`))
      (set `self.IsUsingAbility` true)))
  (:`Ongoing`
    (set `self.AbilityRadius` (select `bool` (<= _returnvalue 499.0) :`false` 500.0 :`true` _returnvalue :!type "Float (single-precision)")))
  (:`Canceled`
    (bind _outhits (`KismetSystemLibrary.SphereTraceMulti` :`Start` _returnvalue_2 :`End` (+ _returnvalue_2 (0.0 0.0 1.0)) :`Radius` (`self.AbilityRadius`) :`TraceChannel` "TraceTypeQuery4" :`DrawDebugType` "ForDuration" :!label _label_2))
    (for _array_element _outhits
      (bind (_bblockinghit _binitialoverlap _time _distance _location _impactpoint _normal _impactnormal _physmat _hitactor _hitcomponent) (`GameplayStatics.BreakHitResult` _array_element))
      (`KismetArrayLibrary.Array_Add` (`self.ArrayofForces`) (* _impactnormal -9000.0))
      (`KismetArrayLibrary.Array_Add` (`self.Hit Component`) _hitcomponent)
      (for (_array_element_2 _array_index) (`self.Hit Component`)
        (`PrimitiveComponent.AddForce` _array_element_2 (`|GetArrayItem` (`self.ArrayofForces`) _array_index) "None" true))
      (if (`self.IsUsingAbility`)
        (set `self.IsUsingAbility` false)
        (set `self.AbilityRadius` 0.0)
        (set `self.ChargeUpTimer` 0.0)
        (`KismetArrayLibrary.Array_Clear` (`self.Hit Component`))
        (`KismetArrayLibrary.Array_Clear` (`self.ArrayofForces`)))))
  (:`Completed`
    (goto _label_2)))

(fn `HitDetection`
  (bind _rootcomponent (`Actor.RootComponent` (`self.AxeGuitar`)))
  (bind _outhit (`KismetSystemLibrary.SphereTraceSingleForObjects` :`Start` (`SceneComponent.GetSocketLocation` _rootcomponent "AxeStart") :`End` (`SceneComponent.GetSocketLocation` _rootcomponent "AxeEnd") :`Radius` 20.0 :`ObjectTypes` (`|MakeArray` "ObjectTypeQuery3" :!type "EObjectTypeQuery Enum") :`DrawDebugType` "ForDuration"))
  (bind _asbp_player_character (cast `/Game/RuWork/Player/BP_PlayerCharacter` (`.HitActor` (`GameplayStatics.BreakHitResult` _outhit))))
  (`self.K2_DestroyActor` _asbp_player_character))

(fn `UserConstructionScript`
  (`parent.UserConstructionScript`))