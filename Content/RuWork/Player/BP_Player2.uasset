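; Second player's character Blueprint, which creates its own per-player HUD and handles pistol fire and pull powers.
; Rate-limited fire switches to aim-facing movement and timer-loops sphere traces that destroy hit BP_PlayerCharacters, with Tick relaxing aim after inactivity.
; Force input activates the GA_Pull gameplay ability.
; Special input sphere-traces from the camera and timeline-lerps the hit actor to PullPoint, toggling physics on grab and release.
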(event `self.ReceiveBeginPlay`
  (`parent.ReceiveBeginPlay`)
  ;[0 0.06699 1] This is to add UI to second palyer
  (`KismetSystemLibrary.Delay` 0.2)
  (bind _asplayer_controller (cast `PlayerController` (`self.GetController`)))
  (bind _returnvalue (`|CreateWidget` "/Game/UI/Players/Player2HUD_Widgit.Player2HUD_Widgit_C" _asplayer_controller))
  (bind _output_get (set `self.HUDRef` _returnvalue))
  (`UserWidget.AddToPlayerScreen` _output_get 0))

(event `self.ReceiveTick`
  (params (DeltaSeconds :type "Float (single-precision)"))
  (if (not (`self.Is Firing`))
    ;[1 0 0] Needs fix for lowering weapon(Lowering gun after shooting for a long time)
    (`self.AimingCheck`)
    (set `self.PullPointLoc` (`SceneComponent.GetSocketLocation` (`self.PullPoint`) "None"))))

(event `EnhancedInput|/Game/Combat/Inputs/IA_PlayerAttack`
  (params (ActionValue :type Boolean) (ElapsedSeconds :type "Float (double-precision)") (TriggeredSeconds :type "Float (double-precision)") (InputAction :type "InputAction Object Reference" :default "/Game/Combat/Inputs/IA_PlayerAttack.IA_PlayerAttack"))
  (bind _charactermovement (`self.CharacterMovement`))
  ;[1 0.4072 0] Fire Pistol - Regular time intervals without access to spamming
  (:`Started`
    (if (>= (- (`KismetSystemLibrary.GetGameTimeInSeconds`) (`self.LastFireTime`)) 0.2)
      (set `self.Is Firing` true)
      (set `self.IsAiming` true)
      (set `CharacterMovementComponent.bOrientRotationToMovement` false _charactermovement)
      (set `CharacterMovementComponent.bUseControllerDesiredRotation` true _charactermovement)
      (`KismetSystemLibrary.K2_SetTimer` null "Shoot" (`self.fireRate`) true)
      (set `self.FireTimer` (struct))
      (set `self.LastFireTime` (`KismetSystemLibrary.GetGameTimeInSeconds`))))
  (:`Completed`
    (`self.Shoot`)
    (set `self.Is Firing` false)
    (`KismetSystemLibrary.K2_ClearAndInvalidateTimerHandle` (`self.FireTimer`))))

(event `EnhancedInput|/Game/Combat/Inputs/IA_ForceAbility`
  (params (ActionValue :type Boolean) (ElapsedSeconds :type "Float (double-precision)") (TriggeredSeconds :type "Float (double-precision)") (InputAction :type "InputAction Object Reference" :default "/Game/Combat/Inputs/IA_ForceAbility.IA_ForceAbility"))
  ;[0.9 0.1664 0] Pulling Ability -> Activates when pressed and pulls enemies towards the player
  (:`Started`
    (if (>= (- (`KismetSystemLibrary.GetGameTimeInSeconds`) (`self.Last Cast Time`)) 0.5)
      (`AbilitySystemComponent.K2_GiveAbilityAndActivateOnce` (`self.AbilitySystem`) "/Game/RuWork/Abilities/GA_Pull.GA_Pull_C" 0 -1)
      (set `self.Last Cast Time` (`KismetSystemLibrary.GetGameTimeInSeconds`)))))

(event `EnhancedInput|/Game/Combat/Inputs/IA_Special`
  (params (ActionValue :type Boolean) (ElapsedSeconds :type "Float (double-precision)") (TriggeredSeconds :type "Float (double-precision)") (InputAction :type "InputAction Object Reference" :default "/Game/Combat/Inputs/IA_Special.IA_Special"))
  (bind _returnvalue (`SceneComponent.K2_GetComponentLocation` (`self.FollowCamera`)))
  (bind _returnvalue_2 (* (`KismetMathLibrary.GetForwardVector` (`self.GetBaseAimRotation`)) (`self.RegisterDistance`)))
  ;[0.9 0.1664 0] Pull Grab -> Grabs objects/players/enemies and drops them when time is up
  (:`Started`
    (if (>= (- (`KismetSystemLibrary.GetGameTimeInSeconds`) (`self.LastCastTime`)) 0.2)
      (set `self.PushDirection` (* _returnvalue_2 -50.0))
      (bind (_outhit _returnvalue_3) (`KismetSystemLibrary.SphereTraceSingle` :`Start` _returnvalue :`End` (+ _returnvalue _returnvalue_2) :`Radius` 30.0 :`TraceChannel` "TraceTypeQuery3" :`DrawDebugType` "ForDuration"))
      (if _returnvalue_3
        (bind (_bblockinghit _binitialoverlap _time _distance _location _impactpoint _normal _impactnormal _physmat _hitactor _hitcomponent) (`GameplayStatics.BreakHitResult` _outhit))
        (set `self.TempLocation` _location)
        (bind _output_get (set `self.IsPlayer` (`KismetMathLibrary.ClassIsChildOf` (`GameplayStatics.GetObjectClass` _hitactor) "/Game/RuWork/Player/BP_PlayerCharacter.BP_PlayerCharacter_C")))
        (if _output_get
          (bind _asbp_player_character (cast `/Game/RuWork/Player/BP_PlayerCharacter` _hitactor))
          (bind _output_get_2 (set `self.Actor` _asbp_player_character))
          (set `self.Hit Component` (`Character.CapsuleComponent` _output_get_2))
          (else
            (set `self.Hit Component` _hitcomponent)))
        (`PrimitiveComponent.SetSimulatePhysics` (`self.Hit Component`) false)
        (bind (_direction _pullcurve) (`Timeline|PullBack` :!via `PlayFromStart` :!label _label)
          (:`Update`
            (`self.K2_SetActorLocation` _hitactor (`KismetMathLibrary.VLerp` (`self.TempLocation`) (`self.PullPointLoc`) _pullcurve) false false))))))
  (:`Canceled`
    (`|ExecutionSequence` :!label _label_2
      (:`then_0`
        (goto _label :!via `Stop`))
      (:`then_1`
        (if (`self.IsPlayer`)
          (`PrimitiveComponent.SetSimulatePhysics` (`self.Hit Component`) true)
          (`KismetSystemLibrary.Delay` 0.3)
          (`PrimitiveComponent.SetSimulatePhysics` (`self.Hit Component`) false)
          (else
            (`PrimitiveComponent.SetSimulatePhysics` (`self.Hit Component`) true))))))
  (:`Completed`
    (goto _label_2)))

(fn `AimingCheck`
  (bind _charactermovement (`self.CharacterMovement`))
  (if (>= (- (`KismetSystemLibrary.GetGameTimeInSeconds`) (`self.LastFireTime`)) 2.0)
    (set `self.IsAiming` false)
    (set `CharacterMovementComponent.bOrientRotationToMovement` true _charactermovement)
    (set `CharacterMovementComponent.bUseControllerDesiredRotation` false _charactermovement)))

(fn `Shoot`
  (bind _returnvalue (`SceneComponent.GetSocketLocation` (`self.SK_Handgun`) "barrel"))
  ;[1 1 1] Fire gun
  (if (`self.Is Firing`)
    (bind _outhit (`KismetSystemLibrary.SphereTraceSingleForObjects` :`Start` _returnvalue :`End` (+ _returnvalue (* (`KismetMathLibrary.GetForwardVector` (`self.GetBaseAimRotation`)) 150000.0)) :`Radius` 5.0 :`ObjectTypes` (`|MakeArray` "ObjectTypeQuery3" :!type "EObjectTypeQuery Enum") :`DrawDebugType` "ForDuration"))
    (bind _asbp_player_character (cast `/Game/RuWork/Player/BP_PlayerCharacter` (`.HitActor` (`GameplayStatics.BreakHitResult` _outhit))))
    (`self.K2_DestroyActor` _asbp_player_character)
    (set `self.LastFireTime` (`KismetSystemLibrary.GetGameTimeInSeconds`))))

(fn `UserConstructionScript`
  (`parent.UserConstructionScript`))